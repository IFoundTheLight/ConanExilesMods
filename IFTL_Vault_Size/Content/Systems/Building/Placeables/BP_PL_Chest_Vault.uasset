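; Vault chest placeable that restricts guild members of Recruit rank from using, dismantling or locking it.
; Overrides the container access, dismantle and lock checks, adding a rank test on top of each parent result through a shared IsRecruit helper.
; Access is denied only to recruits of the owning guild, and creative mode lifts the dismantle restriction.
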(event EventBeginPlay)

(event EventActorBeginOverlap
  (params (OtherActor :type Actor%20Object%20Reference)))

(event EventTick
  (params (DeltaSeconds :type Float%20%28single-precision%29)))

(fn ConstructionScript
  (|CallParentFunction))

(fn CanAccessContainer
  (params (InteractingPawn :type Pawn%20Object%20Reference))
  (bind (_canaccess _containerislocked _instigatorisowner) (|CallParentFunction InteractingPawn))
  (if _canaccess
    (bind _asconan_character (Utilities|Casting|CastToConanCharacter InteractingPawn)
      (:then
        (if (and (CallFunction|IsRecruit _asconan_character) (== (Class|ConanCharacter|GetGuildId _asconan_character) (Variables|Default|GetOwnerUniqueID)))
          (return false _containerislocked _instigatorisowner)
          (else
            _)))
      (:CastFailed
        _)))
  (return _canaccess _containerislocked _instigatorisowner))

(fn GetCanbeDismantled
  (params (DismantlingCharacter :type Conan%20Character%20Object%20Reference))
  (bind _canbedismantled (|CallParentFunction DismantlingCharacter))
  (if _canbedismantled
    (return (or (not (CallFunction|IsRecruit DismantlingCharacter)) (Variables|/Script/ConanSandbox.ConanCharacter|GetbIsInCreativeMode DismantlingCharacter)))
    (else
      (return false))))

(fn IsRecruit
  (params (CharacterToCheck :type Conan%20Character%20Object%20Reference))
  (bind _returnvalue (Class|ConanCharacter|GetGuild CharacterToCheck))
  (bind _characteruniqueid (Variables|/Script/ConanSandbox.ConanCharacter|GetCharacterUniqueID CharacterToCheck))
  (Utilities|IsValid _returnvalue
    (:Is%20Valid
      (Utilities|IsValid _characteruniqueid
        (:Is%20Valid
          (return (Utilities|Enum|Equal(Enum) (Class|Guild|GetPlayerRank _returnvalue _characteruniqueid) "Recruit")))
        (:Is%20Not%20Valid
          _)))
    (:Is%20Not%20Valid
      _))
  (return false))

(fn GetIsLockable
  (params (LockingCharacter :type Conan%20Character%20Object%20Reference))
  (bind _islockable (|CallParentFunction LockingCharacter))
  (if _islockable
    (return (not (CallFunction|IsRecruit LockingCharacter)))
    (else
      (return false))))