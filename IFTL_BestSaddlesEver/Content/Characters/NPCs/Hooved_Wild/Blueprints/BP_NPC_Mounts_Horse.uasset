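; Rideable horse NPC that handles rider brake, jump and rear, speed-based trampling knockback, journey events, and pushing characters out of its body.
; Mane and tail follow the master pose and hide according to the equipped saddle's data table row.
; Server-computed stats, a rare random trait and a timed potion drive replicated male genital visibility and size, gated by nudity settings.
; Listen servers delay setup for database-loaded horses until stats load.
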(event OnComponentBeginOverlap(PushAway)
  (params (OverlappedComponent :type Primitive%20Component%20Object%20Reference) (OtherActor :type Actor%20Object%20Reference) (OtherComp :type Primitive%20Component%20Object%20Reference) (OtherBodyIndex :type Integer) (bFromSweep :type Boolean) (SweepResult :type Hit%20Result%20Structure%20%28by%20ref%29))
  (if (not (or (Variables|Default|GetIsMounted) (Utilities|IsValid (Actor|GetAttachParentActor))))
    (bind _asconan_character (Utilities|Casting|CastToConanCharacter OtherActor))
    (if (and (== (VehicleSound|GetRootComponent _asconan_character) OtherComp) (or (Utilities|DoesObjectImplementInterface _asconan_character "/Game/Systems/Interfaces/BasePlayerCharInterface.BasePlayerCharInterface_C") (Utilities|DoesObjectImplementInterface _asconan_character "/Game/Characters/NPCs/Humanoid/HumanoidNPCInterface.HumanoidNPCInterface_C")))
      (Utilities|Array|AddUnique (Variables|Default|GetCharactersToPushAway) _asconan_character)
      ;[1 1 1] We need this zero tick delay to prevent recursive calls triggered by PushCharacterOut
      (Utilities|FlowControl|Delay 0.0)
      (CallFunction|PushAllCharactersOut))))

(event SignalInventoryRecivedonClient(EquipmentInventory)
  ;[1 1 1] Events to trigger Mane/Tail Show/Hide
  (CallFunction|DisplayMainNTail))

(event SignalItemAdded(EquipmentInventory)
  (params (index :type Integer) (item :type Game%20Item%20Object%20Reference) (srcInventory :type Item%20Inventory%20Object%20Reference) (srcIndex :type Integer))
  ;[1 1 1] Events to trigger Mane/Tail Show/Hide
  (CallFunction|DisplayMainNTail))

(event SignalItemRemoved(EquipmentInventory)
  (params (index :type Integer) (item :type Game%20Item%20Object%20Reference) (dstInventory :type Item%20Inventory%20Object%20Reference) (dstIndex :type Integer))
  ;[1 1 1] Events to trigger Mane/Tail Show/Hide
  (CallFunction|DisplayMainNTail))

(event Custom|SignalItemAdded_PotionOfEndowment
  (params (index :type Integer) (item :type Game%20Item%20Object%20Reference) (srcInventory :type Item%20Inventory%20Object%20Reference) (srcIndex :type Integer))
  (bind _returnvalue (Class|KismetSystemLibrary|MakeLiteralInteger 18275))
  (if (== (Variables|/Script/ConanSandbox.GameItem|GetTemplateID item) _returnvalue)
    (bind _returnvalue_2 (Class|ItemInventory|DeleteItemsbyTemplate (Variables|Default|GetBackpackInventory) _returnvalue "consumed" 1))
    (if _returnvalue_2
      (Utilities|Time|SetTimerbyEvent (delegate Custom|DisablePotionOfEndownment) 6e+01)
      (Variables|Default|SetConsumedPotion true))))

(event Custom|UpdateHorseNudity
  (params (Value :type ENudity%20Enum))
  (if (Math|Boolean|NotEqual(Boolean) (Variables|Default|GetFullNudity) (Utilities|Enum|Equal(Enum) Value "Full"))
    (CallFunction|HandleVisibility)))

(event Custom|CheckIfSaddleWasAdded
  (params (index :type Integer) (item :type Game%20Item%20Object%20Reference) (srcInventory :type Item%20Inventory%20Object%20Reference) (srcIndex :type Integer))
  (if (GameplayTags|DoesContainerMatchTagQuery (Class|GameItem|GetItemGameplayTags item) (GameplayTags|MakeGameplayTagQuery "(TokenStreamVersion=0,TagDictionary=((TagName=\"Item.Saddle.Horse\")),QueryTokenStream=(0,1,2,1,0),UserDescription=\"\",AutoDescription=\" ALL( Item.Saddle.Horse )\")"))
    (bind _returnvalue (Class|ItemInventory|GetConanCharacterOwner srcInventory))
    (Utilities|IsValid _returnvalue
      (:Is%20Valid
        (Class|NewJourneyComponent|AddJourneyEvent (Actor|GetComponentbyClass _returnvalue "/Script/ConanSandbox.NewJourneyComponent") "Outrider_7" (Transformation|GetActorLocation _returnvalue))))))

(event Custom|OnHorseNudityChanged
  (params (NudityLevel :type ENudity%20Enum))
  (CallFunction|UpdateHorseNudity NudityLevel))

(event Custom|DisplayMainNTail
  (bind _inventory (CallFunction|GetEquipmentInventory))
  (bind _returnvalue (Class|EquipmentInventory|GetItematSlot _inventory "PetSaddle"))
  (Utilities|IsValid _returnvalue
    (:Is%20Valid
      (if (not (GameplayTags|DoesContainerMatchTagQuery (Class|GameItem|GetItemGameplayTags _returnvalue) (GameplayTags|MakeGameplayTagQuery "(TokenStreamVersion=0,TagDictionary=((TagName=\"Item.Saddle.Horse\")),QueryTokenStream=(0,1,2,1,0),UserDescription=\"\",AutoDescription=\" ALL( Item.Saddle.Horse )\")")))
        ;[1 1 1] Display the Mane/Tail
        (Development|SetHiddeninGame (Variables|Default|GetTail) false true :!label _label)
        (Development|SetHiddeninGame (Variables|Default|GetMane) false true)
        (else
          (bind _asbpgame_item_saddle (Utilities|Casting|CastToBPGameItem_Saddle _returnvalue))
          (bind (_hidetail _hidemane) (CallFunction|FindSaddleData _asbpgame_item_saddle))
          ;[1 1 1] Show/Hide Mane/Tail
          (Development|SetHiddeninGame (Variables|Default|GetTail) _hidetail true)
          (Development|SetHiddeninGame (Variables|Default|GetMane) _hidemane true))))
    (:Is%20Not%20Valid
      (goto _label))))

(event Custom|HandleVisibility
  (Variables|Default|SetFullNudity (Utilities|Enum|Equal(Enum) (CallFunction|GetClampedNudityLevel) "Full"))
  (Variables|Default|SetShowPenis (Math|Boolean|ANDBoolean (CallFunction|IsGenderMale) (Variables|Default|GetFullNudity) (or (Variables|Default|GetVisibleWithoutPotion) (Variables|Default|GetConsumedPotion))))
  (Variables|Default|SetShowTesticles (Math|Boolean|ANDBoolean (CallFunction|IsGenderMale) (Variables|Default|GetFullNudity) (not (Variables|Default|GetShowPenis))))
  (CallFunction|HandleUpdateSize))

(event Custom|HandleUpdateSize
  (if (not (Networking|IsDedicatedServer))
    (if (or (Variables|Default|GetVisibleWithoutPotion) (Variables|Default|GetConsumedPotion))
      (CallFunction|SetMeshVisibility))
    (if (Variables|Default|GetConsumedPotion)
      (bind (_direction _growthovertime) (Timeline|HorseEndownment Play)
        (:Update
          (Default|UpdateSize (Variables|Default|GetBPI_Horse) (* (Variables|Default|GetEndowmentTarget) _growthovertime)))
        (:Finished
          (switch Utilities|FlowControl|Switch|SwitchonETimelineDirection _direction
            (:Backward
              (CallFunction|SetMeshVisibility)))))
      (else
        (Timeline|HorseEndownment Reverse)))))

(event Custom|SetMeshVisibility
  (bind _penis (Variables|Default|GetPenis))
  (bind _bpi_horse (Variables|Default|GetBPI_Horse))
  (bind _testicles (Variables|Default|GetTesticles))
  (Utilities|FlowControl|Sequence
    (:then_0
      (Utilities|IsValid _penis
        (:Is%20Valid
          (Rendering|SetVisibility _penis (Variables|Default|GetShowPenis) false))))
    (:then_1
      (Utilities|IsInterfaceValid? _bpi_horse
        (:IsValid
          (Default|UpdateVisible _bpi_horse (Variables|Default|GetShowPenis)))))
    (:then_2
      (Utilities|IsValid _testicles
        (:Is%20Valid
          (Rendering|SetVisibility _testicles (Variables|Default|GetShowTesticles) false))))))

(event Custom|DisablePotionOfEndownment
  (Variables|Default|SetConsumedPotion false))

(event Custom|AnimInstanceChanged
  (bind _asbpi_horse_penis (Utilities|Casting|CastToBPI_Horse_Penis (Components|SkeletalMesh|GetAnimInstance (Variables|Character|GetMesh))))
  (Variables|Default|SetBPI_Horse _asbpi_horse_penis)
  (Utilities|FlowControl|Sequence
    (:then_0
      ;[1 1 1] Must run on the server because clients dont know about stats, then we replicate the var
      (if (Networking|IsServer)
        (Utilities|IsValid (Variables|Default|GetStatHolder)
          (:Is%20Valid
            (for _array_element (Variables|Default|GetAttributes)
              (bind _returnvalue (Class|StatHolder|GetIntStatChangeSignal (Variables|Default|GetStatHolder) _array_element))
              (EventDispatchers|BindEventtoSignalStatChanged _returnvalue (delegate Custom|StatChange)))))))
    (:then_1
      (if (not (Networking|IsDedicatedServer)) ; Dedicated servers do not need this
        (Class|SkinnedMeshComponent|SetMasterPoseComponent (Variables|Default|GetPenis) (Variables|Character|GetMesh))
        (Class|SkinnedMeshComponent|SetMasterPoseComponent (Variables|Default|GetTesticles) (Variables|Character|GetMesh))
        (EventDispatchers|BindEventtoOnNudityChanged (Variables|/Script/ConanSandbox.ConanGameState|GetUserSettingsEventDispatcher (.AsConan%20Game%20State (Utilities|Casting|CastToConanGameState (Game|GetGameState)))) (delegate Custom|OnHorseNudityChanged))
        (CallFunction|HandleVisibility)))
    (:then_2
      (if (Networking|IsServer)
        (EventDispatchers|AssignSignalItemAdded (Variables|Default|GetBackpackInventory) (delegate Custom|SignalItemAdded_PotionOfEndowment))))))

(event Custom|StatChange
  (params (actor :type Actor%20Object%20Reference) (statID :type ECharIntStatID%20Enum) (newValue :type Integer) (deltaValue :type Integer))
  ;[1 1 1] Must run on the server because clients dont know about stats, then we replicate the var
  (CallFunction|HandleStatChangeforAttribute))

(event EventBeginPlay
  (bind _inventory (CallFunction|GetEquipmentInventory))
  (|CallParentFunction)
  ;[1 1 1] Attach the horse Mane and Tail
  (for _array_element (Utilities|Array|MakeArray (Variables|Default|GetTail) (Variables|Default|GetMane))
    (Class|SkinnedMeshComponent|SetMasterPoseComponent _array_element (Variables|Character|GetMesh)))
  (if (not (Variables|/Script/UE4Dreamworld.PersistenceComponent|Getm_bWasLoadedFromDB (CallFunction|GetEquipmentInventory)))
    _
    (elif (Class|PersistenceComponent|IsDataDoneLoading _inventory)
      (CallFunction|DisplayMainNTail)
      (else
        (EventDispatchers|BindEventtoOnSignalDataLoaded _inventory (delegate Custom|DisplayMainNTail)))))
  (bind _returnvalue (Class|ConanCharacter|GetActorPersistenceComponent))
  ;[1 1 1] This check if we are on listening server and if the mount was loaded from database. If true, then we have to delay all logic after Stats are loaded (Load NPC in BeginPlay_PersistentStateLoaded in BaseNPC). After loading the stats the Event BeginPlayLoadSuccess is called so we use this to resume the logic on the listening server.
  (Utilities|IsValid _returnvalue
    (:Is%20Valid
      (if (not (Math|Boolean|ANDBoolean (Networking|IsServer) (not (Networking|IsDedicatedServer)) (Variables|/Script/UE4Dreamworld.PersistenceComponent|Getm_bWasLoadedFromDB _returnvalue)))
        (bind _value (CallFunction|IsBeingPlaced :!label _label))
        (if (not _value)
          (Utilities|FlowControl|Sequence
            (:then_0
              (EventDispatchers|BindEventtoOnAnimInstanceClassChanged (Variables|Character|GetMesh) (delegate Custom|AnimInstanceChanged))
              (CallFunction|AnimInstanceChanged))
            (:then_1
              (EventDispatchers|BindEventtoSignalItemAdded (CallFunction|GetEquipmentInventory) (delegate Custom|CheckIfSaddleWasAdded)))))))
    (:Is%20Not%20Valid
      (goto _label))))

(event EventBeginPlayLoadSuccess
  (params (Message :type String))
  ;[1 1 1] This check if we are on listening server and if the mount was loaded from database. If true, then we have to delay all logic after Stats are loaded (Load NPC in BeginPlay_PersistentStateLoaded in BaseNPC). After loading the stats the Event BeginPlayLoadSuccess is called so we use this to resume the logic on the listening server.
  (|CallParentFunction Message)
  (if (Math|Boolean|ANDBoolean (Networking|IsServer) (not (Networking|IsDedicatedServer)) (Variables|/Script/UE4Dreamworld.PersistenceComponent|Getm_bWasLoadedFromDB (stale EventBeginPlay _returnvalue)))
    (bind _value (CallFunction|IsBeingPlaced))
    (if (not _value)
      (Utilities|FlowControl|Sequence
        (:then_0
          (EventDispatchers|BindEventtoOnAnimInstanceClassChanged (Variables|Character|GetMesh) (delegate Custom|AnimInstanceChanged))
          (CallFunction|AnimInstanceChanged))
        (:then_1
          (EventDispatchers|BindEventtoSignalItemAdded (CallFunction|GetEquipmentInventory) (delegate Custom|CheckIfSaddleWasAdded)))))))

(event EventInteractableActivate
  (params (Component :type Primitive%20Component%20Object%20Reference) (Instigator :type Player%20Controller%20Object%20Reference) (HitIndex :type Integer) (TriggeredFromRadialWheel :type Boolean))
  (bind _returnvalue (Pawn|GetControlledPawn Instigator))
  (|CallParentFunction Component Instigator HitIndex TriggeredFromRadialWheel)
  (if (or (.ReturnValue (Class|ConanCharacter|GetEmbeddedSaddleID)) (Utilities|IsValid (Class|EquipmentInventory|GetItematSlot (Variables|Default|GetEquipmentInventory) "PetSaddle")))
    (Class|ExilesJourneyComponent|AddJourneyEvent (Actor|GetComponentbyClass _returnvalue "/Script/ConanSandbox.ExilesJourneyComponent") "RideHorse" (Transformation|GetActorLocation _returnvalue))))

(event EventBrake
  (bind _asbase_player_char_interface (Utilities|Casting|CastToBasePlayerCharInterface (Class|ConanCharacter|GetRider)))
  (Default|PlayMountedAnimation _asbase_player_char_interface "/Game/Characters/NPCs/Horse/animations/AM_horse_brake.AM_horse_brake"))

(event EventJumpActionPressed
  (params (MountInput :type BP%20Mount%20Input%20Object%20Reference))
  (bind _returnvalue (Class|ConanCharacter|GetRider))
  (if (> (Class|MountInput|GetCurrentSpeed MountInput) (Class|MountInput|GetTargetSpeedValue MountInput "WalkingSpeed"))
    (bind _asbase_player_char_interface (Utilities|Casting|CastToBasePlayerCharInterface (Class|ConanCharacter|GetRider)))
    (Default|JumpActionInterface _asbase_player_char_interface true)
    (elif (and (Pawn|Components|CharacterMovement|IsWalking (Variables|/Script/Engine.Character|GetCharacterMovement _returnvalue)) (not (Default|InSubstate (.AsBase%20BPChar (Utilities|Casting|CastToBaseBPChar _returnvalue)) "NewEnumerator21")))
      (bind _asbase_player_char_interface_2 (Utilities|Casting|CastToBasePlayerCharInterface (Class|ConanCharacter|GetRider)))
      (Default|PlayMountedAnimation _asbase_player_char_interface_2 "/Game/Characters/NPCs/Horse/animations/AM_horse_rear_emote.AM_horse_rear_emote" "/Game/Characters/humans/animations/mounted/Horse/AM_human_mounted_rear_horse.AM_human_mounted_rear_horse"))))

(fn ConstructionScript
  (|CallParentFunction)
  (if (Networking|IsDedicatedServer)
    (Components|DestroyComponent (Variables|Default|GetPenis))))

(fn OnRepAttributeCount
  (Variables|Default|SetEndowmentTarget (Math|Float|Clamp(Float) (Math|Float|Power (/ (Variables|Default|GetAttributeCount) (Variables|Default|GetAttributeTarget)) 1e+01)))
  (CallFunction|HandleVisibility))

(fn OnRepConsumedPotion
  (if (not (Networking|IsDedicatedServer))
    (CallFunction|HandleVisibility)))

(fn GenerateGender
  (if (Networking|IsServer)
    (Utilities|IsValid (Variables|Default|GetStatHolder)
      (:Is%20Valid
        (if (== (Class|StatHolder|GetIntStat (Variables|Default|GetStatHolder) "Gender" "Full") 0)
          (Class|StatHolder|SetIntStat (Variables|Default|GetStatHolder) "Gender" (+ 1 (Math|Random|RandomInteger 2)))
          (Class|PersistenceComponent|SetDirty (Variables|Default|GetStatHolder) true 5.0))))))

(fn IsGenderMale
  (switch int (Class|StatHolder|GetIntStat (Variables|Default|GetStatHolder) "Gender" "Full") ; 1 - male\n2 - female
    (:Default
      (CallFunction|GenerateGender)
      (switch int (Class|StatHolder|GetIntStat (Variables|Default|GetStatHolder) "Gender" "Full") ; 1 - male\n2 - female
        (:Default
          (return false))
        (:1
          (CallFunction|GenerateVisibilityWithoutPotion)
          (return true))))
    (:1
      (return true))
    (:2
      (return false))))

(fn PushCharacterOut
  (params (Character :type Conan%20Character%20Object%20Reference))
  (bind _characterpushedoutposition (CallFunction|GetCharacterPushedOutPosition Character))
  (if (< (Math|Vector|VectorLengthSquared (- _characterpushedoutposition (Transformation|GetActorLocation Character))) (Math|Float|Square (Components|Capsule|GetScaledCapsuleRadius (Variables|Default|GetBlock)))) ; Prevent from moving too far away
    (Transformation|SetActorLocation Character _characterpushedoutposition true false)))

(fn GetCharacterPushedOutPosition
  (params (ConanCharacter :type Conan%20Character%20Object%20Reference))
  (LocalVariables|SetLocal_ConanCharacter ConanCharacter)
  (LocalVariables|SetLocal_DistanceVectorToCapsuleAxis (Class|FuncomGenericLibrary|GetDistanceVectortoCapsuleAxis (Transformation|GetActorLocation (LocalVariables|GetLocal_ConanCharacter)) (Variables|Default|GetPushAway)))
  (return (+ (Math|Vector|MakeVector (.X (Math|Vector|BreakVector (* (Math|Vector|Normalize (LocalVariables|GetLocal_DistanceVectorToCapsuleAxis)) (- (+ (Components|Capsule|GetScaledCapsuleRadius (Variables|/Script/Engine.Character|GetCapsuleComponent (LocalVariables|GetLocal_ConanCharacter))) (Variables|/Script/Engine.CapsuleComponent|GetCapsuleRadius (Variables|Default|GetBlock))) (Math|Vector|VectorLength (LocalVariables|GetLocal_DistanceVectorToCapsuleAxis)))))) (.Y (Math|Vector|BreakVector (* (Math|Vector|Normalize (LocalVariables|GetLocal_DistanceVectorToCapsuleAxis)) (- (+ (Components|Capsule|GetScaledCapsuleRadius (Variables|/Script/Engine.Character|GetCapsuleComponent (LocalVariables|GetLocal_ConanCharacter))) (Variables|/Script/Engine.CapsuleComponent|GetCapsuleRadius (Variables|Default|GetBlock))) (Math|Vector|VectorLength (LocalVariables|GetLocal_DistanceVectorToCapsuleAxis)))))) 0.0) (Transformation|GetActorLocation (LocalVariables|GetLocal_ConanCharacter)))))

(fn HandleStatChangeforAttribute
  (for _array_element (Variables|Default|GetAttributes)
    (LocalVariables|Setlocal%20SumAttributeValues (+ (Math|Conversions|ToFloat(Integer) (Class|ConanCharacter|GetIntStat _array_element "Full")) (LocalVariables|Getlocal%20SumAttributeValues))))
  (Variables|Default|SetAttributeCount (+ (LocalVariables|Getlocal%20SumAttributeValues) (Math|Float|SelectFloat 5.0 0.0 (Variables|Default|GetVisibleWithoutPotion)))))

(fn IsBeingPlaced
  (bind _asconan_character (Utilities|Casting|CastToConanCharacter (Components|GetOwner))
    (:then
      (return (and (Variables|/Script/ConanSandbox.ThrallSystemComponent|GetIsPlacingThrall (Class|ConanCharacter|GetThrallSystemComponent _asconan_character)) (== (Variables|/Script/ConanSandbox.ThrallSystemComponent|GetCurrentThrallBrushClass (Class|ConanCharacter|GetThrallSystemComponent _asconan_character)) (Utilities|GetClass self)))))
    (:CastFailed
      (return false))))

(fn GenerateVisibilityWithoutPotion
  (if (Networking|IsServer)
    (bind _output_get (Variables|Default|SetVisibleWithoutPotion (== (Math|Random|RandomIntegerinRange 1 25) 1)))
    (if _output_get
      (bind _returnvalue (Class|ConanCharacter|GetActorPersistenceComponent))
      (Class|PersistenceComponent|SetDirty _returnvalue true 5.0))))

(fn OnRepVisibleWithoutPotion
  (if (not (Networking|IsDedicatedServer))
    (CallFunction|HandleVisibility)))

(fn PushAllCharactersOut
  (for _array_element (Variables|Default|GetCharactersToPushAway)
    (CallFunction|PushCharacterOut _array_element))
  (Utilities|Array|Clear (Variables|Default|GetCharactersToPushAway)))

(fn FindSaddleData
  (params (Saddle :type BP%20Game%20Item%20Saddle%20Object%20Reference))
  (bind (_targetcharacter _riderendurancedamagemodifier _mountendurancedamagemodifier _walkspeed _runspeed _sprintspeed _sprintendurancedrain _swimendurancedrain _enduranceregeneration _accelerationprofileid _hidemane _hidetail) (Utilities|Struct|BreakSaddleTableRow))
  (bind (_targetcharacter_2 _riderendurancedamagemodifier_2 _mountendurancedamagemodifier_2 _walkspeed_2 _runspeed_2 _sprintspeed_2 _sprintendurancedrain_2 _swimendurancedrain_2 _enduranceregeneration_2 _accelerationprofileid_2 _hidemane_2 _hidetail_2) (Utilities|Struct|BreakSaddleTableRow))
  (bind _templateid (Variables|/Script/ConanSandbox.GameItem|GetTemplateID Saddle))
  (bind _returnvalue (Utilities|String|ToString(Integer) _templateid))
  (bind _returnvalue_2 (Utilities|String|StringToName _returnvalue))
  (bind _returnvalue_3 (Utilities|GetDataTableRow "/Game/Items/SaddleTable.SaddleTable" _returnvalue_2)
    (:then
      (return (.HideTail (Utilities|Struct|BreakSaddleTableRow _returnvalue_3)) (.HideMane (Utilities|Struct|BreakSaddleTableRow _returnvalue_3))))
    (:RowNotFound
      (Utilities|GetDataTableRow "/Game/Items/SaddleTable.SaddleTable" _returnvalue_2
        (:then
          (return _hidetail_2 _hidemane_2))
        (:RowNotFound
          (Utilities|GetDataTableRow "/Game/Items/SaddleTable.SaddleTable" _returnvalue_2
            (:then
              (return _hidetail _hidemane))
            (:RowNotFound
              (return false false))))))))

(fn ApplySnowPlowKnockback
  (params (HitResult :type Hit%20Result%20Structure) (SnowPlow :type Scene%20Component%20Object%20Reference))
  (bind _returnvalue (Class|ConanCharacter|GetRider))
  (bind _output_get (LocalVariables|SetLocal_HitResult HitResult))
  (LocalVariables|SetLocal_SnowPlow SnowPlow)
  (bind _asconan_character (Utilities|Casting|CastToConanCharacter (.HitActor (Collision|BreakHitResult _output_get)))
    (:then
      (LocalVariables|SetLocal_KnockbackedCharacter _asconan_character)
      (bind _output_get_2 (LocalVariables|SetLocal_CurrentSpeedSquared (Math|Vector|VectorLengthSquared (Transformation|GetVelocity _returnvalue))))
      (Class|ExilesJourneyComponent|AddJourneyEvent (Actor|GetComponentbyClass _returnvalue "/Script/ConanSandbox.ExilesJourneyComponent") "HorseTackle" (Transformation|GetActorLocation _returnvalue))
      (if (> _output_get_2 (LocalVariables|GetLocal_KnockbackMinSpeed%20))
        (Game|Damage|ApplyDamage (LocalVariables|GetLocal_KnockbackedCharacter) (|CalculateDamageOnKnockBack) (Pawn|GetController (Class|ConanCharacter|GetRider)) self "/Game/Systems/Progression/DmgTypeHealth_BP.DmgTypeHealth_BP_C")
        (CallFunction|MulticastPlaySoundatLocation "/Game/Sound/SFX/Impacts/MountKnockback/sfx_impact_mount_knockback_medium.sfx_impact_mount_knockback_medium" (Transformation|GetActorLocation (LocalVariables|GetLocal_KnockbackedCharacter)))
        (Game|Damage|ApplyPointDamage (LocalVariables|GetLocal_KnockbackedCharacter) 1e+01 (Math|Vector|MakeVector 0.0 0.0 0.0) (LocalVariables|GetLocal_HitResult) (Pawn|GetController) self (select (> (Math|Vector|DotProduct (- (Transformation|GetActorLocation (LocalVariables|GetLocal_KnockbackedCharacter)) (Transformation|GetWorldLocation (LocalVariables|GetLocal_SnowPlow))) (Math|Vector|GetRightVector (LocalVariables|GetLocal_SnowPlow))) 0.0) "/Game/Systems/Combat/DamageTypes/BP_Knockback_Mount_Fast_Right.BP_Knockback_Mount_Fast_Right_C" "/Game/Systems/Combat/DamageTypes/BP_Knockback_Mount_Fast_Left.BP_Knockback_Mount_Fast_Left_C"))
        (return false)
        (elif (> _output_get_2 4.8e+05)
          (CallFunction|MulticastPlaySoundatLocation "/Game/Sound/SFX/Impacts/MountKnockback/sfx_impact_mount_knockback_medium.sfx_impact_mount_knockback_medium" (Transformation|GetActorLocation (LocalVariables|GetLocal_KnockbackedCharacter)))
          (Game|Damage|ApplyPointDamage (LocalVariables|GetLocal_KnockbackedCharacter) 1e+01 (Math|Vector|MakeVector 0.0 0.0 0.0) (LocalVariables|GetLocal_HitResult) (Pawn|GetController) self (select (> (Math|Vector|DotProduct (- (Transformation|GetActorLocation (LocalVariables|GetLocal_KnockbackedCharacter)) (Transformation|GetWorldLocation (LocalVariables|GetLocal_SnowPlow))) (Math|Vector|GetRightVector (LocalVariables|GetLocal_SnowPlow))) 0.0) "/Game/Systems/Combat/DamageTypes/BP_KnockBack_Mount_Slow_Right.BP_KnockBack_Mount_Slow_Right_C" "/Game/Systems/Combat/DamageTypes/BP_KnockBack_Mount_Slow_Left.BP_KnockBack_Mount_Slow_Left_C"))
          (return false)
          (else
            (return false)))))
    (:CastFailed
      (return false))))